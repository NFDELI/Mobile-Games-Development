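; BP_PlatformBase is the base platform in the jump platform game, judging whether a player's jump input matches it.
; On begin play it caches GM_JumpPlatform and, after a short delay, applies the cosmetic platform material from the game mode's loaded data.
; CheckPlayerJump compares the input to the platform's Type; a mismatch makes the game mode's spawner turn off platform collisions.
; A toggle event switches this mesh's collision on or off.
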(event Custom|LoadPlatformSkin
  (Rendering|Material|SetMaterial (Variables|Default|GetPlatformMesh) 0 (Utilities|Struct|BreakF_CosmeticGeneralStructure (.CosmeticStruct (Utilities|Struct|BreakF_SaveStructure (Variables|/Game/JumpPlatform/Blueprints/GM_JumpPlatform.GM_JumpPlatform_C|GetLoadedData (Variables|Default|GetGameModeRef)))))))

(event Custom|ToggleCollisionPreset
  (params (TurnOn? :type Boolean))
  (bind _platformmesh (Variables|Default|GetPlatformMesh))
  (if TurnOn?
    (Collision|SetCollisionEnabled _platformmesh "QueryAndPhysics")
    (else
      (Collision|SetCollisionEnabled _platformmesh "NoCollision"))))

(event EventBeginPlay
  ;[1 0.97 0.97] Begin Play
  (bind _asgm_jump_platform (Utilities|Casting|CastToGM_JumpPlatform (Game|GetGameMode)))
  (Variables|Default|SetGameModeRef _asgm_jump_platform)
  (Utilities|FlowControl|Delay 0.1)
  (CallFunction|LoadPlatformSkin))

(fn ConstructionScript)

(fn CheckPlayerJump
  (params (PlayerInput :type E_PlatformType%20Enum :default "NewEnumerator0"))
  ;[0.01146 0 1] Checks if the player Jump in the correct direction to reach THIS platform.
  (if (Utilities|Enum|Equal(Enum) PlayerInput (Variables|Default|GetType))
    (return true)
    (else
      (Default|TurnOffPlatformsCollisions (Variables|/Game/JumpPlatform/Blueprints/GM_JumpPlatform.GM_JumpPlatform_C|GetPlatformSpawnerRef (Variables|Default|GetGameModeRef)))
      (return false))))