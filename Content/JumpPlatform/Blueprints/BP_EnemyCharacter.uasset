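; BP_EnemyCharacter is the chaser enemy in JumpPlatform, climbing the spawned platforms after the player.
; SpawnChaser places it at a given platform index and starts a self-calling delayed loop that runs while active.
; Each tick teleports it to the next entry in the game mode's platform spawner array, then calls ChaserReachedPlayer on the game mode.
; ChaserIncreaseMoveSpeed shortens the delay between moves.
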(event Custom|SpawnChaser
  (params (SpawnLocation :type Integer))
  (Variables|Default|SetCurrentChaserStep SpawnLocation)
  (CallFunction|TeleportChasertoPlatform)
  (Variables|Default|SetisActive? true)
  (CallFunction|ChaserAITimer))

(event Custom|GetGameModeRef
  (bind _asgm_jump_platform (Utilities|Casting|CastToGM_JumpPlatform (Game|GetGameMode)))
  (Variables|Default|SetGMRef _asgm_jump_platform))

(event Custom|TeleportChaserToPlatform
  (bind _next_platform (CallFunction|GetNextPlatform))
  (bind _returnvalue (Transformation|GetActorTransform _next_platform))
  ;[0.01146 0 1] Teleport Chaser to NEXT platform
  (Transformation|SetActorTransform (Math|Transform|MakeTransform (Math|Vector|MakeVector (.x (.location _returnvalue)) (.y (.location _returnvalue)) (+ (.z (.location _returnvalue)) (Variables|Default|GetChaserModelOffset))) "0, 0, 0" "1.000000,1.000000,1.000000") false true)
  (Math|Integer|IncrementInt (Variables|Default|GetCurrentChaserStep)))

(event Custom|ChaserAITimer
  (if (Variables|Default|GetisActive?)
    (Utilities|FlowControl|Delay (Variables|Default|GetMoveSpeedTimerSeconds)) ; Delay Timer before Chaser Moves up a platform
    (CallFunction|TeleportChasertoPlatform)
    (Default|ChaserReachedPlayer? (Variables|Default|GetGMRef))
    (CallFunction|ChaserAITimer) ; Start the Chaser Move Cycle!
  ))

(event Custom|ChaserIncreaseMoveSpeed
  ;[0 0 1] Increase Chaser Speed.
  (Variables|Default|SetMoveSpeedTimerSeconds (- (Variables|Default|GetMoveSpeedTimerSeconds) (Variables|Default|GetMoveSpeedIncreaseRate))))

(event EventBeginPlay
  (CallFunction|GetGameModeRef))

(fn ConstructionScript)

(fn GetPlatformArray
  (return (Variables|/Game/JumpPlatform/Blueprints/BP_PlatformSpawner.BP_PlatformSpawner_C|GetPlatformArray (Variables|/Game/JumpPlatform/Blueprints/GM_JumpPlatform.GM_JumpPlatform_C|GetPlatformSpawnerRef (Variables|Default|GetGMRef)))))

(fn GetNextPlatform
  (return (Utilities|Array|Get(acopy) (CallFunction|GetPlatformArray) (Variables|Default|GetCurrentChaserStep))))