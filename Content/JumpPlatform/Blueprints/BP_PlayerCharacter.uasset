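; Player character for a left/right platform-jumping game, applying saved skin, hat and jump sound, with swipe-to-rotate cosmetic viewing.
; Each tap asks the next spawned platform to validate direction, then teleports the player onward and updates score, or sideways off the path.
; Death enables gravity, saves score and gold through the GameMode, then polls falling state, correcting out-of-bounds positions, until the PlayerController can show results.
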(event OnComponentBeginOverlap(LandColliderBox)
  (params (OverlappedComponent :type Primitive%20Component%20Object%20Reference) (OtherActor :type Actor%20Object%20Reference) (OtherComp :type Primitive%20Component%20Object%20Reference) (OtherBodyIndex :type Integer) (bFromSweep :type Boolean) (SweepResult :type Hit%20Result%20Structure%20%28by%20ref%29))
  ;[1 0 0.8072] Play Player Landed Sounds
  (bind _astrigger_box (Utilities|Casting|CastToTriggerBox OtherActor))
  (if (not (<= (.z (.location (Transformation|GetActorTransform _astrigger_box))) -1e+02))
    (Audio|PlaySound2D "/Game/JumpPlatform/Sounds/sound_landed.sound_landed" 1.0 1.0 0.05 0 0)
    (else
      (CallFunction|PreventPlayerOutOfBounds false))))

(event Custom|PushedOff
  (if (not (Variables|Default|GetisDead?))
    (CallFunction|PlayerDied)))

(event Custom|TeleportPlayerToNextPlatform
  (bind _nextplatform (CallFunction|GetNextPlatform))
  (bind _returnvalue (Transformation|GetActorTransform _nextplatform))
  ;[0.81 0 0] Teleports the player to the next platform. (This event is called when the player presses the correct direction.)
  (Transformation|SetActorTransform (Math|Transform|MakeTransform (Math|Vector|MakeVector (.x (.location _returnvalue)) (.y (.location _returnvalue)) (+ (.z (.location _returnvalue)) (Variables|Default|GetPlayerZModelOffset))) "0, 0, 0" "1.000000,1.000000,1.000000") false true)
  (CallFunction|PlayStepSound)
  (CallFunction|TeleportAudioVolumetoPlayer))

(event Custom|PlayStepSound
  ;[1 0 0.7362] Play Player Stepping Sounds
  (Audio|PlaySoundatLocation (Variables|Default|GetStepSoundCue) (Transformation|GetActorLocation) "0, 0, 0" 1.0 (Math|Random|RandomFloatinRange 0.9 1.1) 0.0 0 0 0 0))

(event Custom|PlayerJumpsOff
  (params (PlayerInput :type E_PlatformType%20Enum :default "NewEnumerator0"))
  (bind _falloffset (Variables|Default|GetFallOffset))
  ;[0.81 0 0] Player Dies, Jumps off the map.
  (if (Utilities|Enum|Equal(Enum) PlayerInput "NewEnumerator0")
    (bind _result (Utilities|NegateInt _falloffset)
      (:%20%20
        (CallFunction|TeleportPlayertoWrongJumpDirection _result)))
    (else
      (CallFunction|TeleportPlayertoWrongJumpDirection _falloffset)))
  (CallFunction|PlayerDied))

(event Custom|PlayerDied
  (bind _gmref (Variables|References|GetGMRef))
  ;[0 0.1181 1] Player Dying Logic
  (Variables|/Script/Engine.CharacterMovementComponent|SetGravityScale (Variables|Character|GetCharacterMovement) 1.0)
  (Variables|Default|SetisDead? true)
  (Collision|SetCollisionEnabled (Variables|Default|GetLand%20Collider%20Box) "QueryAndPhysics")
  (Default|ToggleArrowTapVisuals (Variables|References|Get%20PCJumpPlatformRef) false)
  (Default|CheckHighscore _gmref)
  (Default|CalculatePlayerGoldEarned _gmref)
  (Default|SaveUpdate _gmref)
  (Utilities|FlowControl|Delay 0.2)
  (CallFunction|CheckPlayerLandedCycle))

(event Custom|CheckPlayerLandedCycle
  ;[0 0.09764 1] Check if Player has Landed
  (if (not (AI|Components|NavMovement|IsFalling (Variables|Character|GetCharacterMovement))) ; Has player reached the ground?
    (Default|TellMainWidgettoShowResults (Variables|References|Get%20PCJumpPlatformRef))
    (else
      (Utilities|FlowControl|Delay 2.0)
      (CallFunction|PreventPlayerOutOfBounds false)
      (CallFunction|CheckPlayerLandedCycle))))

(event Custom|PreventPlayerOutOfBounds
  (params (isTrrigerBoxCalling? :type Boolean))
  (bind _returnvalue (Transformation|GetActorLocation))
  ;[0 0.009266 1] Prevent Player from falling out of Bounds
  (if (CallFunction|IsPlayerY-AxisOutOfBounds?)
    (if isTrrigerBoxCalling?
      (Transformation|SetActorLocation (Math|Vector|MakeVector (.x _returnvalue) 1.75e+03 (.z _returnvalue)) false true)
      (else
        (Transformation|SetActorLocation (Math|Vector|MakeVector (.x (Transformation|GetActorLocation)) 1.75e+03 8e+02) false true :!label _label)))
    (elif (CallFunction|IsPlayerZ-AxisOutOfBounds?)
      (goto _label))))

(event Custom|StartVideoAdAudio
  ;[1 0.005822 0.914] Player VideoAd Sounds
  (CameraShake|Start (Variables|Default|GetMediaSound)))

(event Custom|ResetPlayer
  ;[0 0.03342 1] Reset Player
  (Variables|Default|SetisDead? false)
  (Variables|/Script/Engine.CharacterMovementComponent|SetGravityScale (Variables|Character|GetCharacterMovement) 0.0)
  (Collision|SetCollisionEnabled (Variables|Default|GetLand%20Collider%20Box) "NoCollision")
  (CallFunction|AllowtoDisableMenuArrows)
  (Default|ToggleArrowTapVisuals (Variables|References|Get%20PCJumpPlatformRef) true))

(event Custom|AllowToDisableMenuArrows
  ;[0 1 0] Player Taps Right Arrow (Menu Arrows Disabled here Once because platforms ALWAYS SPAWN RIGHT FIRST )
  (Utilities|FlowControl|DoOnce false) ; enters at Reset
)

(event EventIAJumpRight
  ;[0 1 0] Player Taps Right Arrow (Menu Arrows Disabled here Once because platforms ALWAYS SPAWN RIGHT FIRST )
  (if (not (Variables|Default|GetisDead?))
    (CallFunction|PlayerJumped "NewEnumerator1")
    (Utilities|FlowControl|DoOnce false
      (:Completed
        (Default|DisableMenuArrows (Variables|References|Get%20PCJumpPlatformRef))))))

(event EventBeginPlay
  ;[1 1 1] Begin Play (Get References)
  (bind _asgm_jump_platform (Utilities|Casting|CastToGM_JumpPlatform (Game|GetGameMode)))
  (Variables|References|SetGMRef _asgm_jump_platform)
  (bind _aspc_jump_platform (Utilities|Casting|CastToPC_JumpPlatform (Game|GetPlayerController 0)))
  (Variables|References|Set%20PCJumpPlatformRef _aspc_jump_platform)
  (Utilities|FlowControl|Delay 0.2)
  (CallFunction|LoadSkinTexture (.SkinMaterial (Utilities|Struct|BreakF_CosmeticGeneralStructure (Utilities|Struct|BreakF_SaveStructure (Variables|/Game/JumpPlatform/Blueprints/GM_JumpPlatform.GM_JumpPlatform_C|GetLoadedData (Variables|References|GetGMRef))))))
  (CallFunction|LoadJumpSound (.JumpSound (Utilities|Struct|BreakF_CosmeticGeneralStructure (Utilities|Struct|BreakF_SaveStructure (Variables|/Game/JumpPlatform/Blueprints/GM_JumpPlatform.GM_JumpPlatform_C|GetLoadedData (Variables|References|GetGMRef))))))
  (CallFunction|GetAudioVolumeReference)
  (CallFunction|LoadHatMesh (.HatAsset (Utilities|Struct|BreakF_CosmeticGeneralStructure (Utilities|Struct|BreakF_SaveStructure (Variables|/Game/JumpPlatform/Blueprints/GM_JumpPlatform.GM_JumpPlatform_C|GetLoadedData (Variables|References|GetGMRef))))) (.Scale (Utilities|Struct|BreakF_CosmeticGeneralStructure (Utilities|Struct|BreakF_SaveStructure (Variables|/Game/JumpPlatform/Blueprints/GM_JumpPlatform.GM_JumpPlatform_C|GetLoadedData (Variables|References|GetGMRef))))) (.OffsetLocation (Utilities|Struct|BreakF_CosmeticGeneralStructure (Utilities|Struct|BreakF_SaveStructure (Variables|/Game/JumpPlatform/Blueprints/GM_JumpPlatform.GM_JumpPlatform_C|GetLoadedData (Variables|References|GetGMRef)))))))

(event EventIAJumpLeft
  ;[0 1 0] Player Taps Left Arrow
  (if (not (Variables|Default|GetisDead?))
    (CallFunction|PlayerJumped "NewEnumerator0")))

(event Input|KeyboardEvents|DebugKeyW
  (params (Key :type Key%20Structure :default "None") (ActionValue :type Input%20Action%20Value%20Structure))
  ;[0 0.1181 1] Player Dying Logic
  (:Pressed
    (Development|PrintString (Utilities|String|ToString(Boolean) (AI|Components|NavMovement|IsFalling (Variables|Character|GetCharacterMovement))) true true "(R=0.640000,G=0.000000,B=0.000000,A=1.000000)")))

(event Input|TouchEvents|InputTouch
  (params (Location :type Vector) (FingerIndex :type ETouchIndex%20Enum))
  (bind _returnvalue (Math|Vector2D|MakeVector2D (.x Location) (.y Location)))
  ;[0 1 0 1 48] Cosmetic Model Rotation with Touch
  (:Pressed
    (Variables|CosmeticRotationVariables|SetTouchStartPos _returnvalue)
    (Variables|CosmeticRotationVariables|SetIsTouching? true))
  (:Moved
    (if (Variables|CosmeticRotationVariables|GetIsTouching?)
      (Variables|CosmeticRotationVariables|SetTouchEndPos _returnvalue)
      (Utilities|FlowControl|Sequence
        (:then_0
          (if (CallFunction|CheckSwipeDirectionLeft)
            (Transformation|SetActorRelativeRotation (Math|Rotator|CombineRotators (Transformation|GetActorRotation) (Math|Rotator|MakeRotator 0.0 0.0 (Variables|CosmeticRotationVariables|GetCosmeticViewRotationRate))) :!label _label)
            (else
              (Transformation|SetActorRelativeRotation (Math|Rotator|CombineRotators (Transformation|GetActorRotation) (Math|Rotator|MakeRotator 0.0 0.0 (* (Variables|CosmeticRotationVariables|GetCosmeticViewRotationRate) -1.0))) :!label _label_2))))
        (:then_1
          (if (CallFunction|CheckSwipeDirectionRight)
            (goto _label_2)
            (else
              (goto _label))))))))

(fn ConstructionScript)

(fn GetPlatformsArray
  (return (Variables|/Game/JumpPlatform/Blueprints/BP_PlatformSpawner.BP_PlatformSpawner_C|GetPlatformArray (Variables|/Game/JumpPlatform/Blueprints/GM_JumpPlatform.GM_JumpPlatform_C|GetPlatformSpawnerRef (Variables|References|GetGMRef)))))

(fn TeleportPlayertoWrongJumpDirection
  (params (FallOffset :type Integer))
  (bind _returnvalue (Transformation|GetActorTransform))
  (Transformation|SetActorTransform (Math|Transform|MakeTransform (Math|Vector|MakeVector (.x (.location _returnvalue)) (+ FallOffset (.y (.location _returnvalue))) (+ (.z (.location _returnvalue)) (Variables|Default|GetPlayerZModelOffset))) "0, 0, 0" "1.000000,1.000000,1.000000") false true))

(fn GetNextPlatform
  (return (Utilities|Array|Get(acopy) (CallFunction|GetPlatformsArray) (Variables|/Game/JumpPlatform/Blueprints/GM_JumpPlatform.GM_JumpPlatform_C|GetCurrentPlayerStep (Variables|References|GetGMRef)))))

(fn PlayerJumped
  (params (PlayerInput :type E_PlatformType%20Enum :default "NewEnumerator0"))
  (bind _gmref (Variables|References|GetGMRef))
  ;[0 0 1] Player Jumped, check if the player jumps in the correct direction (Check if anything should happen when the player jumps)
  (bind _isjumpcorrect_ (Default|CheckPlayerJump (CallFunction|GetNextPlatform) PlayerInput))
  (if _isjumpcorrect_
    (CallFunction|TeleportPlayertoNextPlatform)
    (bind _new_player_score (Default|IncreasePlayerScore _gmref))
    (Default|CheckShouldSpawnChaser _gmref)
    (Default|WBScoreUpdate (Variables|/Game/JumpPlatform/Blueprints/Hud/WB_MainHud.WB_MainHud_C|GetWB_PlayerScore (Variables|/Game/JumpPlatform/Blueprints/PC_JumpPlatform.PC_JumpPlatform_C|GetWB_MainHud (Variables|References|Get%20PCJumpPlatformRef))) _new_player_score) ; The Hud updates here!
    (else
      (CallFunction|PlayerJumpsOff PlayerInput)))
  (return))

(fn GetCurrentPlatform)

(fn LoadSkinTexture
  (params (New%20Skin%20Material :type Material%20Instance%20Object%20Reference))
  (Utilities|IsValid New%20Skin%20Material ; Prevents invalid materials to be loaded!
    (:Is%20Valid
      (Rendering|Material|SetMaterial (Variables|Character|GetMesh) 0 New%20Skin%20Material))))

(fn LoadJumpSound
  (params (New%20Jump%20Sound :type Sound%20Cue%20Object%20Reference))
  (Utilities|IsValid New%20Jump%20Sound
    (:Is%20Valid
      (Variables|Default|SetStepSoundCue New%20Jump%20Sound))))

(fn IsPlayerY-AxisOutOfBounds?
  (bind _returnvalue (Transformation|GetActorLocation))
  (return (or (<= (.y _returnvalue) 0.0) (>= (.y _returnvalue) 3.5e+03))))

(fn CheckSwipeDirectionLeft
  (return (> (.x (- (Variables|CosmeticRotationVariables|GetTouchStartPos) (Variables|CosmeticRotationVariables|GetTouchEndPos))) (Variables|CosmeticRotationVariables|GetTouchMoveSensitivity))))

(fn CheckSwipeDirectionRight
  (return (< (.x (- (Variables|CosmeticRotationVariables|GetTouchStartPos) (Variables|CosmeticRotationVariables|GetTouchEndPos))) (* (Variables|CosmeticRotationVariables|GetTouchMoveSensitivity) -1.0))))

(fn GetAudioVolumeReference
  (bind _outactors (Actor|GetAllActorsOfClass "/Script/Engine.AudioVolume"))
  (Variables|Default|SetAudioVolumeRef (Utilities|Array|Get(acopy) _outactors)))

(fn TeleportAudioVolumetoPlayer
  (Transformation|SetActorLocation (Variables|Default|GetAudioVolumeRef) (Transformation|GetActorLocation) false true))

(fn LoadHatMesh
  (params (Hat%20Static%20Mesh :type Static%20Mesh%20Object%20Reference) (Hat%20Scale :type Float%20%28double-precision%29) (Hat%20Offset :type Vector))
  (bind _hat (Variables|Default|GetHat))
  (Components|StaticMesh|SetStaticMesh _hat Hat%20Static%20Mesh)
  (Transformation|SetRelativeScale3D _hat (Math|Vector|MakeVector Hat%20Scale Hat%20Scale Hat%20Scale))
  (Transformation|SetRelativeLocation _hat Hat%20Offset false true))

(fn IsPlayerZ-AxisOutOfBounds?
  (return (<= (.z (Transformation|GetActorLocation)) -1.0)))