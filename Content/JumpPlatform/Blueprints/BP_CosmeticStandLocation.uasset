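; Placed actor that serves as the spot where the player stands while using the cosmetic UI in the JumpPlatform game.
; On BeginPlay it caches the PC_JumpPlatform player controller.
; PlayerGoToCosmeticSpot blends the view to this actor, toggles the cosmetic UI on through that controller, and teleports the controlled pawn to the actor's location with a fixed rotation.
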(event Custom|PlayerGoToCosmeticSpot
  (bind _returnvalue (Game|GetPlayerController 0))
  (Game|Player|SetViewTargetwithBlend _returnvalue self 1.0 "VTBlend_Linear" 0.0 true)
  (Default|ToggleCosmeticUI (Variables|Default|GetPC%20Ref) true)
  (Transformation|SetActorLocationAndRotation (Pawn|GetControlledPawn _returnvalue) (Transformation|GetActorLocation) "0.000000,90.000000,0.000000" false true))

(event EventBeginPlay
  (bind _aspc_jump_platform (Utilities|Casting|CastToPC_JumpPlatform (Game|GetPlayerController 0)))
  (Variables|Default|SetPC%20Ref _aspc_jump_platform))

(fn ConstructionScript)