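; Spawner actor that builds a rising zigzag chain of BP_PlatformBase actors for a jumping game, starting with an initial batch at BeginPlay.
; Each spawn randomly picks left or right, offsets from the last platform in PlatformArray and steps upward; the third type is never rolled.
; It applies the loaded skin material and shows direction arrows on early platforms.
; Events disable all platform collision on death or rebuild the chain.
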(event Custom|SpawnPlatform
  ;[0.01146 0 1] Spawns the Platforms (Spawns either left or right platforms for now)
  (bind _returnvalue (Game|SpawnActorfromClass "/Game/JumpPlatform/Blueprints/BP_PlatformBase.BP_PlatformBase_C" (Math|Transform|MakeTransform (.location (Transformation|GetActorTransform)) "0.000000,180.000000,0.000000" "1.000000,1.000000,1.000000") "Undefined" "MultiplyWithRoot" 0 0))
  (switch int (Math|Random|RandomIntegerinRange 0 1)
    (:0
      (Variables|/Game/JumpPlatform/Blueprints/BP_PlatformBase.BP_PlatformBase_C|SetType _returnvalue "NewEnumerator0")
      (Variables|Default|SetOffsetValue (* (Variables|Default|GetDefaultOffsetValue) -1)))
    (:1
      (Variables|/Game/JumpPlatform/Blueprints/BP_PlatformBase.BP_PlatformBase_C|SetType _returnvalue "NewEnumerator1")
      (Variables|Default|SetOffsetValue (Variables|Default|GetDefaultOffsetValue)))
    (:2
      (Variables|/Game/JumpPlatform/Blueprints/BP_PlatformBase.BP_PlatformBase_C|SetType _returnvalue "NewEnumerator2")))
  (CallFunction|MovePlatform _returnvalue)
  (CallFunction|AddPlatformtoArray _returnvalue)
  (Variables|/Game/JumpPlatform/Blueprints/BP_PlatformBase.BP_PlatformBase_C|SetPlatfromSkinMat _returnvalue (Variables|Default|GetPlatformMaterial))
  (CallFunction|SetArrowGuideDirection _returnvalue))

(event Custom|AddPlatformToArray
  (params (PlatformToAdd :type BP%20Platform%20Base%20Object%20Reference))
  ;[0.81 0 0 1 15] Adds the Platform to the Array (Makes sure that its Unique)
  (Utilities|Array|AddUnique (Variables|Default|GetPlatformArray) PlatformToAdd) ; Make sure that the platform is not the exact same Platform Instance
)

(event Custom|MovePlatform
  (params (PlatformToMove :type BP%20Platform%20Base%20Object%20Reference))
  (bind _platformarray (Variables|Default|GetPlatformArray))
  (bind _returnvalue (Utilities|Array|LastIndex _platformarray))
  (bind _output (Utilities|Array|Get(acopy) _platformarray _returnvalue))
  (bind _returnvalue_2 (Transformation|GetActorTransform _output))
  ;[0.81 0 0] Moves the Platform to the correct Offset (Either left offset or right offset)
  (if (== (Utilities|Array|Length (Variables|Default|GetPlatformArray)) 0) ; The first Platform does not need to be offset!
    (Variables|/Game/JumpPlatform/Blueprints/BP_PlatformBase.BP_PlatformBase_C|SetType PlatformToMove "NewEnumerator1") ; The first platform must always jump right.
    (else
      (Transformation|SetActorTransform PlatformToMove (Math|Transform|MakeTransform (Math|Vector|MakeVector (.x (.location _returnvalue_2)) (+ (.y (.location _returnvalue_2)) (Variables|Default|GetOffsetValue)) (+ (.z (.location _returnvalue_2)) 1.2e+02)) "0.000000,180.000000,0.000000" "1.000000,1.000000,1.000000") false true))))

(event Custom|TurnOffPlatformsCollisions
  ;[0.01146 0 1] Turn off ALL platform collisions. (Called when player dies)
  (for _array_element (Variables|Default|GetPlatformArray)
    (Default|ToggleCollisionPreset _array_element false)))

(event Custom|SetArrowGuideDirection
  (params (PlatformToMove :type BP%20Platform%20Base%20Object%20Reference))
  (bind _jumpdirectionguide (Variables|/Game/JumpPlatform/Blueprints/BP_PlatformBase.BP_PlatformBase_C|GetJumpDirectionGuide PlatformToMove))
  (if (<= (Utilities|Array|LastIndex (Variables|Default|GetPlatformArray)) (Variables|Default|GetNumOfGuidePlatforms))
    (if (Utilities|Enum|Equal(Enum) (Variables|/Game/JumpPlatform/Blueprints/BP_PlatformBase.BP_PlatformBase_C|GetType PlatformToMove) "NewEnumerator0")
      (Transformation|SetRelativeRotation _jumpdirectionguide "0.000000,0.000000,-180.000000" false false))
    (Rendering|SetVisibility _jumpdirectionguide true false)))

(event Custom|LoadPlatformMat
  (params (NewPlatformMaterial :type Material%20Instance%20Object%20Reference))
  (Variables|Default|SetPlatformMaterial NewPlatformMaterial))

(event Custom|ResetPlatforms
  (bind _platformarray (Variables|Default|GetPlatformArray))
  (for _array_element _platformarray
    (Actor|DestroyActor _array_element))
  (Utilities|Array|Clear _platformarray)
  (CallFunction|SpawnInitialPlatforms))

(event Custom|SpawnInitialPlatforms
  (for _index (range 1 (Variables|Default|GetNumOfInitialPlatforms)) ; Change the last index to determine how many platforms spawns
    (CallFunction|SpawnPlatform)))

(event EventBeginPlay
  ;[1 1 1] Begin Play sets how many paltforms to spawn.
  (Variables|Default|SetOffsetValue (Variables|Default|GetDefaultOffsetValue))
  (CallFunction|SpawnInitialPlatforms))

(fn ConstructionScript)