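; BP_DistractionSpawnLocation is a movable spawner actor that spawns distraction birds near the player in the JumpPlatform game.
; On BeginPlay it caches the GM_JumpPlatform game mode to reach the player reference.
; Each SpawnBird call randomly picks left or right, teleports the spawner to a raised side offset from the player, then spawns a BP_Bird yawed to match that side and prints a debug message.
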(event Custom|UpdateSpawnerLocation
  (if (Variables|Default|GetisSpawningLeft?)
    (Variables|Default|SetOffsetFromPlayer "0.000000,-675.000000,550.000000")
    (else
      (Variables|Default|SetOffsetFromPlayer "0.000000,675.000000,550.000000")))
  (Transformation|SetActorLocation (+ (Transformation|GetActorLocation (Variables|/Game/JumpPlatform/Blueprints/GM_JumpPlatform.GM_JumpPlatform_C|GetPlayerRef (Variables|Default|GetGM%20Ref))) (Variables|Default|GetOffsetFromPlayer)) false true))

(event Custom|InitGameModeRef
  ;[1 1 1] Initialize Game Mode Reference
  (bind _asgm_jump_platform (Utilities|Casting|CastToGM_JumpPlatform (Game|GetGameMode)))
  (Variables|Default|SetGM%20Ref _asgm_jump_platform))

(event Custom|SpawnBirdPawn
  (Variables|Default|SetisSpawningLeft? (Math|Random|RandomBool))
  (CallFunction|UpdateSpawnerLocation)
  (if (Variables|Default|GetisSpawningLeft?)
    (Variables|Default|SetZRotation 9e+01)
    (else
      (Variables|Default|SetZRotation -9e+01)))
  (Game|SpawnActorfromClass "/Game/JumpPlatform/Blueprints/BP_Bird.BP_Bird_C" (Math|Transform|MakeTransform (Transformation|GetActorLocation) (Math|Rotator|MakeRotator 0.0 0.0 (Variables|Default|GetZRotation)) "1.000000,1.000000,1.000000") "AlwaysSpawn" "MultiplyWithRoot" 0 0)
  (Development|PrintString "BIRD SPAWNED"))

(event EventBeginPlay
  (CallFunction|InitGameModeRef))

(event EventSpawnBird
  (CallFunction|SpawnBirdPawn))

(fn ConstructionScript)