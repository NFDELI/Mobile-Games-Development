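; BP_Bird is a bird actor for the JumpPlatform game that plays a looping wing-flap animation.
; BeginPlay starts PlayBirdAnimationCycle, which uses short delays to step the wings through middle, down, middle and high poses, then calls itself to repeat.
; The flap is a visibility swap: three helper functions each show one of the BirdUp, BirdMiddle and BirdDown components and hide the other two.
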(event Custom|PlayBirdAnimationCycle
  ;[1 1 1] Bird Flying Animation
  (Utilities|FlowControl|Delay 0.12)
  (CallFunction|SetBirdWingstoMiddle)
  (Utilities|FlowControl|Delay 0.13)
  (CallFunction|SetBirdWingstoDown)
  (Utilities|FlowControl|Delay 0.13)
  (CallFunction|SetBirdWingstoMiddle)
  (Utilities|FlowControl|Delay 0.12)
  (CallFunction|SetBirdWingstoHigh)
  (CallFunction|PlayBirdAnimationCycle))

(event EventBeginPlay
  (CallFunction|PlayBirdAnimationCycle))

(fn ConstructionScript)

(fn SetBirdWingstoMiddle
  (Rendering|SetVisibility (Variables|Default|GetBirdUp) false false)
  (Rendering|SetVisibility (Variables|Default|GetBirdMiddle) true false)
  (Rendering|SetVisibility (Variables|Default|GetBirdDown) false false)
  (return))

(fn SetBirdWingstoDown
  (Rendering|SetVisibility (Variables|Default|GetBirdUp) false false)
  (Rendering|SetVisibility (Variables|Default|GetBirdMiddle) false false)
  (Rendering|SetVisibility (Variables|Default|GetBirdDown) true false)
  (return))

(fn SetBirdWingstoHigh
  (Rendering|SetVisibility (Variables|Default|GetBirdUp) true false)
  (Rendering|SetVisibility (Variables|Default|GetBirdMiddle) false false)
  (Rendering|SetVisibility (Variables|Default|GetBirdDown) false false)
  (return))