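; Player controller for the JumpPlatform game that turns left and right jump input into messages for the controlled pawn.
; On BeginPlay it adds the Enhanced Input mapping context to player 0's subsystem and, if that subsystem is valid, caches the game instance.
; The left and right jump actions call message functions on the pawn, leaving the jump logic itself to the pawn.
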(event Input|EnhancedActionEvents|EnhancedInputActionIA_LeftJump
  (params (ActionValue :type Boolean) (ElapsedSeconds :type Float%20%28double-precision%29) (TriggeredSeconds :type Float%20%28double-precision%29) (InputAction :type Input%20Action%20Object%20Reference :default "/Game/JumpPlatform/Inputs/IA_LeftJump.IA_LeftJump"))
  (:Triggered
    (Class|BIInputs|IAJumpLeft(Message) (Pawn|GetControlledPawn))))

(event Input|EnhancedActionEvents|EnhancedInputActionIA_RIghtJump
  (params (ActionValue :type Boolean) (ElapsedSeconds :type Float%20%28double-precision%29) (TriggeredSeconds :type Float%20%28double-precision%29) (InputAction :type Input%20Action%20Object%20Reference :default "/Game/JumpPlatform/Inputs/IA_RIghtJump.IA_RIghtJump"))
  (:Triggered
    (Class|BIInputs|IAJumpRight(Message) (Pawn|GetControlledPawn))))

(event EventBeginPlay
  (bind _aspc_jump_platform (Utilities|Casting|CastToPC_JumpPlatform (Game|GetPlayerController 0)))
  (Utilities|IsValid (PlayerController|LocalPlayerSubsystems|GetEnhancedInputLocalPlayerSubsystem _aspc_jump_platform)
    (:Is%20Valid
      (Input|AddMappingContext (PlayerController|LocalPlayerSubsystems|GetEnhancedInputLocalPlayerSubsystem _aspc_jump_platform) "/Game/JumpPlatform/Inputs/IMC_JumpPlatform.IMC_JumpPlatform" 0 "(bIgnoreAllPressedKeysUntilRelease=True,bForceImmediately=False)")
      (bind _asgi_jump_platform (Utilities|Casting|CastToGI_JumpPlatform (Game|GetGameInstance)))
      (Variables|Default|SetGame%20Instance%20Ref _asgi_jump_platform))))

(fn ConstructionScript)