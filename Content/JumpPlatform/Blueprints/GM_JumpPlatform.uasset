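; Game mode for the jump-platform game, managing run progress, scoring, gold, skins and saving.
; BeginPlay waits a tick, loads or creates the single save slot and caches spawner, player, chaser and cosmetic-spot actors.
; Player steps drive batched platform spawning and chaser speed-ups, with separate events for chaser spawn and catch checks.
; High score, step-based gold, skins and volume settings persist through BP_Save, with loaded values messaged to the player controller.
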(event Custom|TellChaserToSpawn
  ;[0 1 0] Chaser Spawn, check if the conditions are met to spawn the chaser.
  (if (not (Variables|Default|GetisChaserSpawned?))
    (Default|SpawnChaser (Variables|References|GetChaserRef) 7)
    (Variables|Default|SetisChaserSpawned? true)))

(event Custom|GetPlatformSpawnerReference
  ;[0 0 0] Get References
  (bind _returnvalue (Actor|GetActorOfClass "/Game/JumpPlatform/Blueprints/BP_PlatformSpawner.BP_PlatformSpawner_C"))
  (Variables|References|SetPlatformSpawnerRef _returnvalue))

(event Custom|GetChaserReference
  ;[0 0 0] Get References
  (bind _returnvalue (Actor|GetActorOfClass "/Game/JumpPlatform/Blueprints/BP_EnemyCharacter.BP_EnemyCharacter_C"))
  (Variables|References|SetChaserRef _returnvalue))

(event Custom|ChaserReachedPlayer?
  ;[1 0 0] Checks if the Chaser Cought the Player
  (if (>= (Variables|/Game/JumpPlatform/Blueprints/BP_EnemyCharacter.BP_EnemyCharacter_C|GetCurrentChaserStep (Variables|References|GetChaserRef)) (Variables|ScoreVariables|GetCurrentPlayerStep))
    (Default|PushedOff (Variables|References|GetPlayerRef)) ; Player Dies in a different way than pressing the wrong jump direction.
    (Variables|/Game/JumpPlatform/Blueprints/BP_EnemyCharacter.BP_EnemyCharacter_C|SetisActive? (Variables|References|GetChaserRef) false) ; Make Chaser Stop Moving.
  ))

(event Custom|CheckShouldIncreaseChaserSpeed
  (bind _result (Math|Integer|IncrementInt (Variables|StepsTo|GetStepsToIncreaseChaserSpeed))
    (:%20%20
      (if (>= _result (Variables|PlayerStepsUntil|GetPlayerStepUntilChaserIncreaseMoveSpeed))
        (Variables|StepsTo|SetStepsToIncreaseChaserSpeed 0)
        (Default|ChaserIncreaseMoveSpeed (Variables|References|GetChaserRef))))))

(event Custom|CheckShouldSpawnMorePlatforms
  ;[0.81 0 0] Check to see if more Platforms are needed to be spawned.
  (bind _result (Math|Integer|IncrementInt (Variables|StepsTo|GetStepsToIncreasePlatform))
    (:%20%20
      (if (>= _result 6)
        (CallFunction|TellSpawnertoSpawnMorePlatforms)
        (Variables|StepsTo|SetStepsToIncreasePlatform 0)))))

(event Custom|CalculatePlayerGoldEarned
  (bind _currentplayerstep (Variables|ScoreVariables|GetCurrentPlayerStep))
  (bind _minimumscoretogaingold (Variables|GoldVariables|GetMinimumScoreToGainGold))
  (bind _returnvalue (/ _currentplayerstep _minimumscoretogaingold))
  ;[0.01146 0 1] CalculatePlayerGoldEarned (Calculate the amount of Gold the Player can earn if Possible AND adds the gold amount.)
  (if (>= _returnvalue 1)
    (bind _output_get (Variables|GoldVariables|SetGold%20Earned _returnvalue))
    (Variables|GoldVariables|SetPlayerGold (+ _output_get (Variables|GoldVariables|GetPlayerGold)))))

(event Custom|TeleportPlayerToCosmeticSpot
  ;[0.01146 0 1] TeleportPlayerToCosmeticSpot (Can be replaced with walking animation)
  (Transformation|SetActorLocation (Variables|References|GetPlayerRef) (Transformation|GetActorLocation (Variables|References|GetCosmeticSpotRef)) false true))

(event Custom|GetCosmeticSpotReference
  ;[0 0 0] Get References
  (bind _returnvalue (Actor|GetActorOfClass "/Game/JumpPlatform/Blueprints/BP_CosmeticStandLocation.BP_CosmeticStandLocation_C"))
  (Variables|References|SetCosmeticSpotRef _returnvalue))

(event Custom|SaveSettings
  (bind _bpsaveref (Variables|References|GetBPSaveRef))
  ;[0.01146 0 1] Save System (Called in the Begin Play as well)
  (bind _returnvalue (SaveGame|DoesSaveGameExist "Save One")) ; The name "Save One" is Important!
  (if _returnvalue
    (Variables|/Game/JumpPlatform/Blueprints/BP_Save.BP_Save_C|SetMasterVolumeValueSave _bpsaveref (Variables|Settings|GetMasterVolumeValue))
    (Variables|/Game/JumpPlatform/Blueprints/BP_Save.BP_Save_C|SetSFXVolumeValueSave _bpsaveref (Variables|Settings|GetSFXVolumeValue))
    (SaveGame|SaveGametoSlot _bpsaveref "Save One")))

(event Custom|StartUpSaveLoad
  ;[0.01146 0 1] Save System (Called in the Begin Play as well)
  (bind _returnvalue (SaveGame|DoesSaveGameExist "Save One")) ; The name "Save One" is Important!
  (if _returnvalue
    (CallFunction|LoadSetUp)
    (else
      (CallFunction|SaveSetUp))))

(event Custom|GetGameInstanceReference
  ;[0 0 0] Get References
  (bind _asgi_jump_platform (Utilities|Casting|CastToGI_JumpPlatform (Game|GetGameInstance))
    (:then
      (Variables|References|SetGameInstanceRef _asgi_jump_platform))
    (:CastFailed
      (Development|PrintString "From GameMode: Failed to get GI Ref"))))

(event Custom|PlayWinBackgroundSound
  (Audio|PlaySound2D "/Game/JumpPlatform/Sounds/wind-outside-sound-ambient-141989.wind-outside-sound-ambient-141989" 1.0 1.0 0.0 0 0))

(event Custom|LoadSaveFile
  (bind _bpsaveref (Variables|References|GetBPSaveRef))
  ;[0.01146 0 1] Save System (Called in the Begin Play as well)
  (bind _returnvalue (SaveGame|DoesSaveGameExist "Save One")) ; This makes sure BPSaveRef is NOT a NULL reference.
  (if _returnvalue
    (Variables|ScoreVariables|SetHighScore (Variables|/Game/JumpPlatform/Blueprints/BP_Save.BP_Save_C|GetHighScoreSave _bpsaveref))
    (Variables|GoldVariables|SetPlayerGold (Variables|/Game/JumpPlatform/Blueprints/BP_Save.BP_Save_C|GetPlayerGoldSave _bpsaveref))))

(event Custom|GetPlayerReference
  ;[0 0 0] Get References
  (bind _returnvalue (Actor|GetActorOfClass "/Game/JumpPlatform/Blueprints/BP_PlayerCharacter.BP_PlayerCharacter_C"))
  (Variables|References|SetPlayerRef _returnvalue))

(event Custom|CheckHighscore
  (bind _currentplayerstep (Variables|ScoreVariables|GetCurrentPlayerStep))
  (if (> _currentplayerstep (Variables|/Game/JumpPlatform/Blueprints/BP_Save.BP_Save_C|GetHighScoreSave (Variables|References|GetBPSaveRef)))
    (Variables|ScoreVariables|SetHighScore _currentplayerstep)))

(event Custom|CheckShouldSpawnChaser
  ;[0 1 0] Chaser Spawn, check if the conditions are met to spawn the chaser.
  (if (>= (Variables|ScoreVariables|GetCurrentPlayerStep) (Variables|PlayerStepsUntil|GetPlayerStepUntilChaserSpawns))
    (CallFunction|TellChasertoSpawn)))

(event Custom|TellSpawnerToSpawnMorePlatforms
  ;[0 1 0 1 14] Tell the Platform Spawner to Spawn more Platforms. (The 'Last Index' determines how many platforms will spawn)
  (for _index (range 0 10)
    (Default|SpawnPlatform (Variables|References|GetPlatformSpawnerRef))))

(event EventBeginPlay
  ;[1 1 1] Begin Play (Call Get References)
  (Utilities|FlowControl|DelayUntilNextTick)
  (CallFunction|GetGameInstanceReference)
  (CallFunction|StartUpSaveLoad)
  (CallFunction|GetPlatformSpawnerReference)
  (CallFunction|GetPlayerReference)
  (CallFunction|GetChaserReference)
  (CallFunction|GetCosmeticSpotReference)
  (CallFunction|PlayWinBackgroundSound))

(event EventUpdateEquippedSkinID
  (params (New%20Skin%20ID :type Integer))
  (Variables|Default|SetSkinEquippedID New%20Skin%20ID)
  (Default|LoadSkinTexture (Variables|References|GetPlayerRef)))

(event EventSaveGame
  (CallFunction|SaveUpdate))

(event EventReducePlayerGold
  (params (Reduce%20Gold%20by :type Integer))
  (Variables|GoldVariables|SetPlayerGold (- (Variables|GoldVariables|GetPlayerGold) Reduce%20Gold%20by))
  (CallFunction|SaveUpdate) ; To Save Gold Data
  (bind _aspc_jump_platform (Utilities|Casting|CastToPC_JumpPlatform (Game|GetPlayerController 0)))
  (Default|LoadGoldUI _aspc_jump_platform))

(event EventAddSkinIDasOwned
  (params (Newly%20Owned%20Skin%20ID :type Integer))
  (Utilities|Array|AddUnique (Variables|Default|GetOwnedSkinsArray) Newly%20Owned%20Skin%20ID))

(fn ConstructionScript)

(fn IncreasePlayerScore
  (bind _result (Math|Integer|IncrementInt (Variables|ScoreVariables|GetCurrentPlayerStep))
    (:%20%20
      (CallFunction|CheckShouldSpawnMorePlatforms)
      (CallFunction|CheckShouldIncreaseChaserSpeed)
      (return _result))))

(fn LoadSetUp
  (bind _returnvalue (Game|GetPlayerController 0))
  (bind _returnvalue_2 (SaveGame|LoadGamefromSlot "Save One"))
  (bind _asbp_save (Utilities|Casting|CastToBP_Save _returnvalue_2))
  (Variables|References|SetBPSaveRef _asbp_save)
  (Variables|ScoreVariables|SetHighScore (Variables|/Game/JumpPlatform/Blueprints/BP_Save.BP_Save_C|GetHighScoreSave _asbp_save))
  (Variables|GoldVariables|SetPlayerGold (Variables|/Game/JumpPlatform/Blueprints/BP_Save.BP_Save_C|GetPlayerGoldSave _asbp_save))
  (Variables|Default|SetSkinEquippedID (Variables|/Game/JumpPlatform/Blueprints/BP_Save.BP_Save_C|GetEquippedSkinID _asbp_save))
  (bind _output_get (Variables|Default|SetOwnedSkinsArray (Variables|/Game/JumpPlatform/Blueprints/BP_Save.BP_Save_C|GetOwnedSkinsArray _asbp_save)))
  (Variables|Settings|SetMasterVolumeValue (Variables|/Game/JumpPlatform/Blueprints/BP_Save.BP_Save_C|GetMasterVolumeValueSave _asbp_save))
  (Variables|Settings|SetSFXVolumeValue (Variables|/Game/JumpPlatform/Blueprints/BP_Save.BP_Save_C|GetSFXVolumeValueSave _asbp_save))
  (Class|BIItemSlotInteraction|LoadOwnedSkinsStatusItemSlot(Message) _returnvalue _output_get)
  (Class|BIItemSlotInteraction|LoadEquippedSkinStatusItemSlot(Message) _returnvalue (Variables|Default|GetSkinEquippedID))
  (Class|BISettingsInteraction|LoadSettingValues(Message) _returnvalue (Variables|Settings|GetMasterVolumeValue) (Variables|Settings|GetSFXVolumeValue))
  (Development|PrintString "Save is Loaded!")
  (return))

(fn SaveSetUp
  (bind _returnvalue (SaveGame|CreateSaveGameObject "/Game/JumpPlatform/Blueprints/BP_Save.BP_Save_C"))
  (Variables|/Game/JumpPlatform/Blueprints/BP_Save.BP_Save_C|SetHighScoreSave _returnvalue 0)
  (Variables|/Game/JumpPlatform/Blueprints/BP_Save.BP_Save_C|SetPlayerGoldSave _returnvalue 0)
  (Variables|/Game/JumpPlatform/Blueprints/BP_Save.BP_Save_C|SetEquippedSkinID _returnvalue 1)
  (Utilities|Array|SetArrayElem (Variables|/Game/JumpPlatform/Blueprints/BP_Save.BP_Save_C|GetOwnedSkinsArray _returnvalue) 0 1 true)
  (SaveGame|SaveGametoSlot _returnvalue "Save One")
  (Variables|References|SetBPSaveRef _returnvalue)
  (return))

(fn SaveUpdate
  (bind _bpsaveref (Variables|References|GetBPSaveRef))
  (bind _returnvalue (SaveGame|DoesSaveGameExist "Save One")) ; The name "Save One" is Important!
  (if _returnvalue
    (Variables|/Game/JumpPlatform/Blueprints/BP_Save.BP_Save_C|SetHighScoreSave _bpsaveref (Variables|ScoreVariables|GetHighScore))
    (Variables|/Game/JumpPlatform/Blueprints/BP_Save.BP_Save_C|SetPlayerGoldSave _bpsaveref (Variables|GoldVariables|GetPlayerGold))
    (Variables|/Game/JumpPlatform/Blueprints/BP_Save.BP_Save_C|SetEquippedSkinID _bpsaveref (Variables|Default|GetSkinEquippedID))
    (Variables|/Game/JumpPlatform/Blueprints/BP_Save.BP_Save_C|SetOwnedSkinsArray _bpsaveref (Variables|Default|GetOwnedSkinsArray))
    (Variables|/Game/JumpPlatform/Blueprints/BP_Save.BP_Save_C|SetMasterVolumeValueSave _bpsaveref (Variables|Settings|GetMasterVolumeValue))
    (Variables|/Game/JumpPlatform/Blueprints/BP_Save.BP_Save_C|SetSFXVolumeValueSave _bpsaveref (Variables|Settings|GetSFXVolumeValue))
    (SaveGame|SaveGametoSlot _bpsaveref "Save One")
    (Development|PrintString "Game is Saved!")))

(fn GetPlayerGold
  (return 0))